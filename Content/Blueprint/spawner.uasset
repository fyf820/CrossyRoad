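; Road spawner actor that creates Highway actors, starting with one at a fixed location on BeginPlay.
; Spawnroad records each new Highway as NewestRoad and hands it a reference back to the spawner.
; Every Tick, SpawnInitialRoad loops to spawn several more roads at NewestRoad's root component location, falling back to the player pawn's location when NewestRoad is invalid.
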(event `self.ReceiveBeginPlay`
  (`self.spawnroad` (-500.0 -300.0 0.0)))

(event `self.ReceiveTick`
  (params (DeltaSeconds :type "Float (single-precision)"))
  (`self.SpawnInitialRoad`))

(fn `SpawnInitialRoad`
  (for _ (range 3)
    (`/Engine/EditorBlueprintResources/StandardMacros.IsValid` (`self.NewestRoad`)
      (:`Is Valid`
        (`self.SpawnRoadAtSpawnPoint`))
      (:`Is Not Valid`
        (`self.spawnroad` (`self.K2_GetActorLocation` (`GameplayStatics.GetPlayerPawn` 0)))))))

(fn `spawnroad`
  (params (SpawnLocation :type "Vector Structure"))
  (bind _returnvalue (`|SpawnActorFromClass` "/Game/StaticObject/highway.highway_C" (`KismetMathLibrary.MakeTransform` SpawnLocation) "Undefined" "OverrideRootScale" null null))
  (bind _output_get (set `self.NewestRoad` _returnvalue))
  (set `/Game/StaticObject/highway.RoadSpawner` self _output_get))

(fn `SpawnRoadAtSpawnPoint`
  (`self.spawnroad` (`SceneComponent.K2_GetComponentLocation` (`Actor.RootComponent` (`self.NewestRoad`)))))

(fn `UserConstructionScript`)