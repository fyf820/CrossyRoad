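; Player-controlled chicken character that walks, jumps with a cluck and can be killed by cars or an eagle.
; Axis input feeds scaled movement input, which Tick consumes and applies directly as an unswept local offset on the Chicken component.
; Four rotate actions snap that component to fixed facings.
; Death functions hide it, play a sound and spawn Deadchick; only the car death disables collision, and DeadByWater is empty.
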(event `self.ReceiveTick`
  (params (DeltaSeconds :type "Float (single-precision)"))
  (bind _returnvalue (`self.ConsumeMovementInputVector`))
  (`SceneComponent.K2_AddLocalOffset` (`self.Chicken`) _returnvalue false false))

(event `InputAxis|MoveForward`
  (params (AxisValue :type "Float (single-precision)"))
  (`self.AddMovementInput` (`self.GetActorForwardVector`) (* AxisValue (`self.speed`))))

(event `InputAction|Jump`
  (params (Key :type "Key Structure"))
  (:`Pressed`
    (`self.Jump`)
    (`GameplayStatics.PlaySoundAtLocation` "/Game/sound/buck.buck" (`SceneComponent.K2_GetComponentLocation` (`self.Chicken`)) (struct) 1.0 1.0 0.0 null null null))
  (:`Released`
    (`self.StopJumping`)))

(event `InputAction|RotateForward`
  (params (Key :type "Key Structure"))
  (:`Pressed`
    (`SceneComponent.K2_SetWorldRotation` :`self` (`self.Chicken`))))

(event `InputAxis|MoveRight`
  (params (AxisValue :type "Float (single-precision)"))
  (`self.AddMovementInput` (`self.GetActorRightVector`) (* (`self.speed`) AxisValue)))

(event `InputAction|RotateLeft`
  (params (Key :type "Key Structure"))
  (:`Pressed`
    (`SceneComponent.K2_SetWorldRotation` (`self.Chicken`) (struct :`Yaw` -90.0) false false)))

(event `InputAction|RotateRight`
  (params (Key :type "Key Structure"))
  (:`Pressed`
    (`SceneComponent.K2_SetWorldRotation` (`self.Chicken`) (struct :`Yaw` 90.0) false false)))

(event `InputAction|RotateBackword`
  (params (Key :type "Key Structure"))
  (:`Pressed`
    (`SceneComponent.K2_SetWorldRotation` (`self.Chicken`) (struct :`Yaw` 180.0) false false)))

(fn `Dead by Car`
  (bind _returnvalue (`SceneComponent.K2_GetComponentLocation` (`self.Chicken`)))
  (`|SpawnActorFromClass` "/Game/StaticObject/deadchick.deadchick_C" (`KismetMathLibrary.Conv_VectorToTransform` _returnvalue) "AlwaysSpawn" "OverrideRootScale" null null)
  (`GameplayStatics.PlaySoundAtLocation` "/Game/sound/chickendeath.chickendeath" _returnvalue (struct) 1.0 1.0 0.0 null null null)
  (`SceneComponent.SetVisibility` (`self.Chicken`) false false)
  (`PrimitiveComponent.SetCollisionEnabled` (`self.Chicken`) "NoCollision"))

(fn `DeadByEagle`
  (`GameplayStatics.PlaySoundAtLocation` "/Game/sound/chickendeath.chickendeath" (`SceneComponent.K2_GetComponentLocation` (`self.Chicken`)) (struct) 1.0 1.0 0.0 null null null)
  (`SceneComponent.SetVisibility` (`self.Chicken`) false false)
  (`|SpawnActorFromClass` "/Game/StaticObject/deadchick.deadchick_C" (`SceneComponent.K2_GetComponentToWorld` (`self.Chicken`)) "Undefined" "OverrideRootScale" null null))

(fn `DeadByWater`)

(fn `UserConstructionScript`)