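; Game mode that procedurally builds an endless chain of terrain tiles: road, rail, water and two highway variants.
; BeginPlay spawns a road, then every Tick spawns a batch of randomly chosen tiles, with no limit or cleanup.
; Each spawn function places its tile at NextSpawnPoint, then advances it to that tile's spawn-point component.
; The Ishighway flag makes a highway run open with Highway1 and continue with Highway2.
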(event `self.ReceiveBeginPlay`
  (`self.SpawnRoad`))

(event `self.ReceiveTick`
  (params (DeltaSeconds :type "Float (single-precision)"))
  (for _ (range 11)
    (switch `int` (`KismetMathLibrary.RandomIntegerInRange` 0 3)
      (:`0`
        (`self.SpawnRoad`)
        (set `self.ishighway` false))
      (:`1`
        (`self.SpawnRail`)
        (set `self.ishighway` false))
      (:`2`
        (`self.SpawnWater`)
        (set `self.ishighway` false))
      (:`3`
        (if (`self.ishighway`)
          (`self.SpawnRoad2`)
          (set `self.ishighway` true)
          (else
            (`self.SpawnRoad1`)
            (set `self.ishighway` true)))))))

(fn `SpawnRail`
  (bind _returnvalue (`|SpawnActorFromClass` "/Game/StaticObject/railroad.railroad_C" (`self.NextSpawnPoint`) "Undefined" "OverrideRootScale" null null))
  (bind _asrailroad (cast `/Game/StaticObject/railroad` _returnvalue))
  (set `self.NextSpawnPoint` (`KismetMathLibrary.MakeTransform` (`SceneComponent.K2_GetComponentLocation` (`/Game/StaticObject/railroad.SpawnPoint` _asrailroad)))))

(fn `SpawnRoad`
  (bind _returnvalue (`|SpawnActorFromClass` "/Game/StaticObject/Road.Road_C" (`self.NextSpawnPoint`) "Undefined" "OverrideRootScale" null null))
  (bind _asroad (cast `/Game/StaticObject/Road` _returnvalue))
  (set `self.NextSpawnPoint` (`KismetMathLibrary.MakeTransform` (`SceneComponent.K2_GetComponentLocation` (`/Game/StaticObject/Road.SpawnPoint` _asroad)))))

(fn `SpawnRoad1`
  (bind _returnvalue (`|SpawnActorFromClass` "/Game/StaticObject/highway1.highway1_C" (`self.NextSpawnPoint`) "Undefined" "OverrideRootScale" null null))
  (bind _ashighway_1 (cast `/Game/StaticObject/highway1` _returnvalue))
  (set `self.NextSpawnPoint` (`KismetMathLibrary.MakeTransform` (`SceneComponent.K2_GetComponentLocation` (`/Game/StaticObject/highway1.SpawnPoint` _ashighway_1)))))

(fn `SpawnRoad2`
  (bind _returnvalue (`|SpawnActorFromClass` "/Game/StaticObject/highway2.highway2_C" (`self.NextSpawnPoint`) "Undefined" "OverrideRootScale" null null))
  (bind _ashighway_2 (cast `/Game/StaticObject/highway2` _returnvalue))
  (set `self.NextSpawnPoint` (`KismetMathLibrary.MakeTransform` (`SceneComponent.K2_GetComponentLocation` (`/Game/StaticObject/highway2.SpawnPoint` _ashighway_2)))))

(fn `SpawnWater`
  (bind _returnvalue (`|SpawnActorFromClass` "/Game/StaticObject/water.water_C" (`self.NextSpawnPoint`) "Undefined" "OverrideRootScale" null null))
  (bind _aswater (cast `/Game/StaticObject/water` _returnvalue))
  (set `self.NextSpawnPoint` (`KismetMathLibrary.MakeTransform` (`SceneComponent.K2_GetComponentLocation` (`/Game/StaticObject/water.SpwanPoint` _aswater)))))

(fn `UserConstructionScript`)